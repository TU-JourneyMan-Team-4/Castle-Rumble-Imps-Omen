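; Candle flame actor for a chandelier prop that turns about the vertical axis to face the player camera.
; Tick runs through a short Delay, throttling the billboard update, then sets rotation from the normalized camera direction with height zeroed out.
; A Fall event destroys the actor.
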(event `self.ReceiveTick`
  (params (DeltaSeconds :type "Float (single-precision)"))
  (`KismetSystemLibrary.Delay` 0.1)
  (`self.K2_SetActorRotation` (`KismetMathLibrary.Conv_VectorToRotator` (`KismetMathLibrary.Normal` (* (- (`PlayerCameraManager.GetCameraLocation` (`GameplayStatics.GetPlayerCameraManager` 0)) (`self.K2_GetActorLocation`)) (1.0 1.0 0.0))))))

(event `Fall`
  (`self.K2_DestroyActor`))

(fn `UserConstructionScript`)