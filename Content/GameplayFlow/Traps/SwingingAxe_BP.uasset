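; Swinging axe trap whose pivot starts moving automatically after play begins.
; BeginPlay builds left, right and start rotations from the pivot's world yaw, then one timeline rotates it from start to left.
; That timeline's updates trigger, after a delay, a second timeline rotating between left and right.
; An Interact overlap toggles the player's HUD press-E prompt, but no interaction or damage logic is implemented here.
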(event `self.ReceiveBeginPlay`
  (bind (_returnvalue_roll _returnvalue_pitch _returnvalue_yaw) (`KismetMathLibrary.BreakRotator` (`SceneComponent.K2_GetComponentRotation` (`self.Pivot`))))
  (`|ExecutionSequence`
    (:`then_0`
      (set `self.Left` (`KismetMathLibrary.MakeRotator` 0.0 60.0 _returnvalue_yaw))
      (set `self.Right` (`KismetMathLibrary.MakeRotator` 0.0 -60.0 _returnvalue_yaw))
      (set `self.Start` (`KismetMathLibrary.MakeRotator` 0.0 0.0 _returnvalue_yaw)))
    (:`then_1`
      ;[1 1 1] Figuring this bit out
      (`KismetSystemLibrary.Delay` 0.3)
      (bind (_direction _newtrack_1) (`Timeline|Timeline_0`)
        (:`Update`
          (`SceneComponent.K2_SetWorldRotation` (`self.Pivot`) (`KismetMathLibrary.RLerp` (`self.Start`) (`self.Left`) _newtrack_1) false false)
          (`KismetSystemLibrary.Delay` 0.3)
          (bind (_direction_2 _newtrack_1_2) (`Timeline|Timeline_1`)
            (:`Update`
              (`SceneComponent.K2_SetWorldRotation` (`self.Pivot`) (`KismetMathLibrary.RLerp` (`self.Left`) (`self.Right`) _newtrack_1_2) false false))))))))

(event `self.ReceiveTick`
  (params (DeltaSeconds :type "Float (single-precision)"))
  ;[1 1 1] Figuring this bit out
)

(event `self.Interact.OnComponentBeginOverlap`
  (params (OverlappedComponent :type "PrimitiveComponent Object Reference") (OtherActor :type "Actor Object Reference") (OtherComp :type "PrimitiveComponent Object Reference") (OtherBodyIndex :type Integer) (bFromSweep :type Boolean) (SweepResult :type "HitResult Structure (by ref)"))
  (if (`self.ActorHasTag` OtherActor "Player")
    (`/Game/UI/HUD.press e` (`/Game/Player/Player.HUD` (cast `/Game/Player/Player` OtherActor :!pure true)))))

(event `self.Interact.OnComponentEndOverlap`
  (params (OverlappedComponent :type "PrimitiveComponent Object Reference") (OtherActor :type "Actor Object Reference") (OtherComp :type "PrimitiveComponent Object Reference") (OtherBodyIndex :type Integer))
  (if (`self.ActorHasTag` OtherActor "Player")
    (`/Game/UI/HUD.Press e no` (`/Game/Player/Player.HUD` (cast `/Game/Player/Player` OtherActor :!pure true)))))

(fn `NewFunction_0`)

(fn `UserConstructionScript`)