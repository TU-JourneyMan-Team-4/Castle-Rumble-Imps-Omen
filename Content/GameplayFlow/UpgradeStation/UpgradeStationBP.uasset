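; Upgrade station actor that lets the player open an upgrade shop UI while in range.
; Overlapping the Interact component shows a press-E prompt on the player's HUD and sets PlayerInReach.
; OpenUpgradeStation resets and shows the player's Upgrade UI, enables the cursor, sets InShop and hides the prompt.
; Leaving the overlap hides the UI, cursor and prompt, and clears both flags.
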(event `Open UpgradeStation`
  (bind _asplayer (cast `/Game/Player/Player` (`GameplayStatics.GetPlayerCharacter` 0) :!pure true))
  (bind _upgrade (`/Game/Player/Player.Upgrade` _asplayer))
  (`/Game/UI/Widgets/UpgradeWidget.ResetUI` _upgrade)
  (`/Game/UI/Widgets/UpgradeWidget.Upgrade Visible` _upgrade)
  (set `PlayerController.bShowMouseCursor` true (`GameplayStatics.GetPlayerController` 0))
  (set `/Game/Player/Player.inShop` true _asplayer)
  (`/Game/UI/Widgets/HUD.Press e no` (`/Game/Player/Player.HUD` (cast `/Game/Player/Player` (`GameplayStatics.GetPlayerCharacter` 0) :!pure true)) :!label _label))

(event `self.Interact.OnComponentBeginOverlap`
  (params (OverlappedComponent :type "PrimitiveComponent Object Reference") (OtherActor :type "Actor Object Reference") (OtherComp :type "PrimitiveComponent Object Reference") (OtherBodyIndex :type Integer) (bFromSweep :type Boolean) (SweepResult :type "HitResult Structure (by ref)"))
  (`/Game/UI/Widgets/HUD.press e` (`/Game/Player/Player.HUD` (cast `/Game/Player/Player` OtherActor :!pure true)))
  (set `self.playerInReach` true))

(event `self.Interact.OnComponentEndOverlap`
  (params (OverlappedComponent :type "PrimitiveComponent Object Reference") (OtherActor :type "Actor Object Reference") (OtherComp :type "PrimitiveComponent Object Reference") (OtherBodyIndex :type Integer))
  (`/Game/UI/Widgets/UpgradeWidget.Upgrade Hidden` (`/Game/Player/Player.Upgrade` (cast `/Game/Player/Player` OtherActor :!pure true)))
  (set `PlayerController.bShowMouseCursor` false (`GameplayStatics.GetPlayerController` 0))
  (set `/Game/Player/Player.inShop` false (cast `/Game/Player/Player` (`GameplayStatics.GetPlayerCharacter` 0) :!pure true))
  (set `self.playerInReach` false)
  (goto _label))

(fn `UserConstructionScript`)