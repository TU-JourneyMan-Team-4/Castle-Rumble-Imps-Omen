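; Omen Alter objective station that summons objectives and pays out the player's pending gold, silver or bronze reward.
; TriggerRewardStation and its duplicate DiningHall request an objective from ObjectiveManager when unlocked and no reward is pending, otherwise calling GiveReward.
; GiveReward locks the altar, then adds random tier loot to the inventory or spawns a pickup if full.
; Colour, light and sword visibility show state; overlap shows HUD prompts.
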(event `Reward Not Available`
  (`MeshComponent.SetVectorParameterValueOnMaterials` (`self.StaticMesh`) "Colour" (1.0 0.27 0.0))
  (`LightComponent.SetLightColor` (`self.PointLight1`) (struct :`R` 1.0 :`G` 0.27 :`A` 1.0) true))

(event `Cooldown Enable`
  (`MeshComponent.SetVectorParameterValueOnMaterials` (`self.StaticMesh`) "Colour" (0.0 0.0 0.0))
  (`SceneComponent.SetVisibility` (`self.Sword1`) false false)
  (`SceneComponent.SetVisibility` (`self.Sword`) false false)
  (`LightComponent.SetLightColor` (`self.PointLight1`) (struct :`A` 1.0) true)
  (set `self.objectivesLocked` true))

(event `Reward Available`
  (`MeshComponent.SetVectorParameterValueOnMaterials` (`self.StaticMesh`) "Colour" (0.0 1.0 0.0))
  (`LightComponent.SetLightColor` (`self.PointLight1`) (struct :`G` 1.0 :`A` 1.0) true))

(event `Cooldown Disable`
  (`MeshComponent.SetVectorParameterValueOnMaterials` (`self.StaticMesh`) "Colour" (1.0 0.27 0.0))
  (`SceneComponent.SetVisibility` (`self.Sword1`) true false)
  (`SceneComponent.SetVisibility` (`self.Sword`) true false)
  (`LightComponent.SetLightColor` (`self.PointLight1`) (struct :`R` 1.0 :`G` 0.27 :`A` 1.0) true)
  (set `self.objectivesLocked` false))

(event `Objective In Progress`
  (`MeshComponent.SetVectorParameterValueOnMaterials` (`self.StaticMesh`) "Colour" (1.0 0.0 0.0))
  (`SceneComponent.SetVisibility` (`self.Sword1`) false false)
  (`SceneComponent.SetVisibility` (`self.Sword`) false false)
  (`LightComponent.SetLightColor` (`self.PointLight1`) (struct :`R` 1.0 :`A` 1.0) true))

(event `GiveReward`
  (params (RewardDictionary :type "Map of /Game/Player/Equipment/Equipment Enum to Integer"))
  (bind _asplayer (cast `/Game/Player/Player` (`GameplayStatics.GetPlayerCharacter` 0) :!pure true))
  (`self.Cooldown Enable`)
  (bind _isfull (`/Game/Player/Player.func_IsInventoryFull` _asplayer))
  (bind _keys (`BlueprintMapLibrary.Map_Keys` RewardDictionary))
  (if _isfull
    (bind _output (`|GetArrayItem` _keys (`KismetMathLibrary.RandomIntegerInRange` 0 (- (`KismetArrayLibrary.Array_Length` _keys) 1))))
    (switch `/Game/Player/Equipment/Equipment` _output
      (:`NewEnumerator5`
        (set `self.equipmentToDrop` "/Game/Player/Equipment/Pickups/ImpShiv_pickup2.ImpShiv_pickup2_C"))
      (:`NewEnumerator3`
        (set `self.equipmentToDrop` "/Game/Player/Equipment/Pickups/Fireball_pickup2.Fireball_pickup2_C"))
      (:`NewEnumerator4`
        (set `self.equipmentToDrop` "/Game/Player/Equipment/Pickups/Crossbow_pickup2.Crossbow_pickup2_C"))
      (:`NewEnumerator1`
        (set `self.equipmentToDrop` "/Game/Player/Equipment/Pickups/Whip_pickup2.Whip_pickup2_C"))
      (:`NewEnumerator6`
        (set `self.equipmentToDrop` "/Game/Player/Equipment/Pickups/MonsterRepellent_pickup2.MonsterRepellent_pickup2_C"))
      (:`NewEnumerator7`
        (set `self.equipmentToDrop` "/Game/Player/Equipment/Pickups/CorruptedHalo_pickup2.CorruptedHalo_pickup2_C"))
      (:`NewEnumerator8`
        (set `self.equipmentToDrop` "/Game/Player/Equipment/Pickups/UnholyCross_pickup2.UnholyCross_pickup2_C"))
      (:`NewEnumerator9`
        (set `self.equipmentToDrop` "/Game/Player/Equipment/Pickups/SpeedPotion_pickup2.SpeedPotion_pickup2_C"))
      (:`NewEnumerator10`
        (set `self.equipmentToDrop` "/Game/Player/Equipment/Pickups/HealthPotion_pickup2.HealthPotion_pickup2_C"))
      (:`NewEnumerator12`
        (set `self.equipmentToDrop` "/Game/Player/Equipment/Pickups/FireRune_pickup.FireRune_pickup_C"))
      (:`NewEnumerator13`
        (set `self.equipmentToDrop` "/Game/Player/Equipment/Pickups/HealthRune_pickup.HealthRune_pickup_C"))
      (:`NewEnumerator14`
        (set `self.equipmentToDrop` "/Game/Player/Equipment/Pickups/IceRune_pickup.IceRune_pickup_C"))
      (:`NewEnumerator15`
        (set `self.equipmentToDrop` "/Game/Player/Equipment/Pickups/TimeRune_pickup.TimeRune_pickup_C"))
      (:`NewEnumerator16`
        (set `self.equipmentToDrop` "/Game/Player/Equipment/Pickups/TeleportRune_pickup.TeleportRune_pickup_C")))
    (bind _returnvalue (`|SpawnActorFromClass` (`self.equipmentToDrop`) (`SceneComponent.K2_GetComponentToWorld` (`self.SpawnAnchor`)) "Undefined" "OverrideRootScale" null null))
    (bind _value (`BlueprintMapLibrary.Map_Find` RewardDictionary _output))
    (set `/Game/Player/Equipment/Pickups/PickUpbase.NumEquipment` _value (cast `/Game/Player/Equipment/Pickups/PickUpbase` _returnvalue :!pure true))
    (`self.Reward Not Available`)
    (else
      (`/Game/Player/Player.func_AddToInventory` _asplayer _output _value)
      (`self.Reward Not Available`))))

(event `TriggerRewardStation`
  (bind _asplayer (cast `/Game/Player/Player` (`GameplayStatics.GetPlayerCharacter` 0) :!pure true))
  (bind _pendingreward (`/Game/Player/Player.pendingReward` _asplayer))
  (if (`|EnumEquality` _pendingreward "NewEnumerator3")
    (if (not (`self.objectivesLocked`))
      (bind _returnvalue (`GameplayStatics.GetActorOfClass` "/Game/GameplayFlow/Objectives/ObjectiveManager.ObjectiveManager_C"))
      (`/Game/GameplayFlow/Objectives/ObjectiveManager.RequestObjective` _returnvalue)
      (`self.Objective In Progress`))
    (elif (`|EnumEquality` _pendingreward "NewEnumerator0")
      (`self.GiveReward` (`self.goldRewards`))
      (set `/Game/Player/Player.pendingReward` "NewEnumerator3" _asplayer :!label _label)
      (`/Game/UI/Widgets/HUD.Reward Text Set` (`/Game/Player/Player.HUD` _asplayer))
      (elif (`|EnumEquality` _pendingreward "NewEnumerator1")
        (`self.GiveReward` (`self.silverRewards`))
        (goto _label)
        (elif (`|EnumEquality` _pendingreward "NewEnumerator2")
          (`self.GiveReward` (`self.bronzeRewards`))
          (goto _label))))))

(event `Dining Hall`
  (bind _asplayer (cast `/Game/Player/Player` (`GameplayStatics.GetPlayerCharacter` 0) :!pure true))
  (bind _pendingreward (`/Game/Player/Player.pendingReward` _asplayer))
  (if (`|EnumEquality` _pendingreward "NewEnumerator3")
    (if (not (`self.objectivesLocked`))
      (bind _returnvalue (`GameplayStatics.GetActorOfClass` "/Game/GameplayFlow/Objectives/ObjectiveManager.ObjectiveManager_C"))
      (`/Game/GameplayFlow/Objectives/ObjectiveManager.RequestObjective` _returnvalue)
      (`self.Objective In Progress`))
    (elif (`|EnumEquality` _pendingreward "NewEnumerator0")
      (`self.GiveReward` (`self.goldRewards`))
      (set `/Game/Player/Player.pendingReward` "NewEnumerator3" _asplayer :!label _label_2)
      (`/Game/UI/Widgets/HUD.Reward Text Set` (`/Game/Player/Player.HUD` _asplayer))
      (elif (`|EnumEquality` _pendingreward "NewEnumerator1")
        (`self.GiveReward` (`self.silverRewards`))
        (goto _label_2)
        (elif (`|EnumEquality` _pendingreward "NewEnumerator2")
          (`self.GiveReward` (`self.bronzeRewards`))
          (goto _label_2))))))

(event `self.Interact.OnComponentBeginOverlap`
  (params (OverlappedComponent :type "PrimitiveComponent Object Reference") (OtherActor :type "Actor Object Reference") (OtherComp :type "PrimitiveComponent Object Reference") (OtherBodyIndex :type Integer) (bFromSweep :type Boolean) (SweepResult :type "HitResult Structure (by ref)"))
  (bind _hud (`/Game/Player/Player.HUD` (cast `/Game/Player/Player` OtherActor :!pure true)))
  (if (`self.ActorHasTag` OtherActor "Player")
    (if (`self.objectivesLocked`)
      (`/Game/UI/Widgets/HUD.Description` _hud "Visible" "Omen Alter" "Come back next round.")
      (else
        (`/Game/UI/Widgets/HUD.Description` _hud "Visible" "Omen Alter" "Summon an Objective.")))))

(event `self.Interact.OnComponentEndOverlap`
  (params (OverlappedComponent :type "PrimitiveComponent Object Reference") (OtherActor :type "Actor Object Reference") (OtherComp :type "PrimitiveComponent Object Reference") (OtherBodyIndex :type Integer))
  (if (`self.ActorHasTag` OtherActor "Player")
    (`/Game/UI/Widgets/HUD.Description` (`/Game/Player/Player.HUD` (cast `/Game/Player/Player` OtherActor :!pure true)) "Hidden" "" "")))

(fn `UserConstructionScript`)