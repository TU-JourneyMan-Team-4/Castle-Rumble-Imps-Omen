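; Reward station where the player requests objectives and collects pending gold, silver or bronze rewards, with an overlap-driven interact prompt.
; TriggerRewardStation reads the player's PendingReward, either requesting an objective from ObjectiveManager or granting a random item from that tier's array with a tier-based quantity.
; Items go into the inventory, or spawn as pickups at SpawnAnchor when it is full.
; Two point lights change color to show station state.
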(event `Reward Not Available`
  (`LightComponent.SetLightColor` (`self.PointLight`) (struct :`R` 1.0 :`G` 0.786581 :`A` 1.0) true)
  (`LightComponent.SetLightColor` (`self.PointLight1`) (struct :`R` 1.0 :`G` 0.786581 :`A` 1.0) true))

(event `Objective In Progress`
  (`LightComponent.SetLightColor` (`self.PointLight`) (struct :`R` 1.0 :`G` 0.000203 :`A` 1.0) true)
  (`LightComponent.SetLightColor` (`self.PointLight1`) (struct :`R` 1.0 :`G` 0.000203 :`A` 1.0) true))

(event `Reward Available`
  (`LightComponent.SetLightColor` (`self.PointLight`) (struct :`G` 1.0 :`B` 0.071519 :`A` 1.0) true)
  (`LightComponent.SetLightColor` (`self.PointLight1`) (struct :`G` 1.0 :`B` 0.071519 :`A` 1.0) true))

(event `GiveReward`
  (params (RewardArray :type "Array of /Game/Player/Equipment/Equipment Enum") (RewardAmount :type Integer))
  (bind _asplayer (cast `/Game/Player/Player` (`GameplayStatics.GetPlayerCharacter` 0) :!pure true))
  (bind _output (`|GetArrayItem` RewardArray (`KismetMathLibrary.RandomIntegerInRange` 0 (- (`KismetArrayLibrary.Array_Length` RewardArray) 1))))
  (bind _isfull (`/Game/Player/Player.IsInventoryFull` _asplayer))
  (if _isfull
    (switch `/Game/Player/Equipment/Equipment` _output
      (:`NewEnumerator5`
        (set `self.equipmentToDrop` "/Game/Player/Equipment/Pickups/ImpShiv_pickup2.ImpShiv_pickup2_C"))
      (:`NewEnumerator3`
        (set `self.equipmentToDrop` "/Game/Player/Equipment/Pickups/Fireball_pickup2.Fireball_pickup2_C"))
      (:`NewEnumerator4`
        (set `self.equipmentToDrop` "/Game/Player/Equipment/Pickups/Crossbow_pickup2.Crossbow_pickup2_C"))
      (:`NewEnumerator1`
        (set `self.equipmentToDrop` "/Game/Player/Equipment/Pickups/Whip_pickup2.Whip_pickup2_C"))
      (:`NewEnumerator17`
        (set `self.equipmentToDrop` "/Game/Player/Equipment/Pickups/VampireHand_pickup.VampireHand_pickup_C"))
      (:`NewEnumerator6`
        (set `self.equipmentToDrop` "/Game/Player/Equipment/Pickups/MonsterRepellent_pickup2.MonsterRepellent_pickup2_C"))
      (:`NewEnumerator7`
        (set `self.equipmentToDrop` "/Game/Player/Equipment/Pickups/CorruptedHalo_pickup2.CorruptedHalo_pickup2_C"))
      (:`NewEnumerator8`
        (set `self.equipmentToDrop` "/Game/Player/Equipment/Pickups/UnholyCross_pickup2.UnholyCross_pickup2_C"))
      (:`NewEnumerator9`
        (set `self.equipmentToDrop` "/Game/Player/Equipment/Pickups/SpeedPotion_pickup2.SpeedPotion_pickup2_C"))
      (:`NewEnumerator10`
        (set `self.equipmentToDrop` "/Game/Player/Equipment/Pickups/HealthPotion_pickup2.HealthPotion_pickup2_C"))
      (:`NewEnumerator12`
        (set `self.equipmentToDrop` "/Game/Player/Equipment/Pickups/FireRune_pickup.FireRune_pickup_C"))
      (:`NewEnumerator13`
        (set `self.equipmentToDrop` "/Game/Player/Equipment/Pickups/HealthRune_pickup.HealthRune_pickup_C"))
      (:`NewEnumerator14`
        (set `self.equipmentToDrop` "/Game/Player/Equipment/Pickups/IceRune_pickup.IceRune_pickup_C"))
      (:`NewEnumerator15`
        (set `self.equipmentToDrop` "/Game/Player/Equipment/Pickups/TimeRune_pickup.TimeRune_pickup_C"))
      (:`NewEnumerator16`
        (set `self.equipmentToDrop` "/Game/Player/Equipment/Pickups/TeleportRune_pickup.TeleportRune_pickup_C"))
      (:`NewEnumerator18`
        (set `self.equipmentToDrop` "/Game/Player/Equipment/Pickups/SoulCrystal_pickup.SoulCrystal_pickup_C")))
    (bind _returnvalue (`|SpawnActorFromClass` (`self.equipmentToDrop`) (`SceneComponent.K2_GetComponentToWorld` (`self.SpawnAnchor`)) "Undefined" "OverrideRootScale" null null))
    (set `/Game/Player/Equipment/Pickups/PickUpbase.NumEquipment` RewardAmount (cast `/Game/Player/Equipment/Pickups/PickUpbase` _returnvalue :!pure true))
    (`self.Reward Not Available`)
    (else
      (`/Game/Player/Player.func_AddToInventory` _asplayer _output RewardAmount)
      (`self.Reward Not Available`))))

(event `TriggerRewardStation`
  (bind _asplayer (cast `/Game/Player/Player` (`GameplayStatics.GetPlayerCharacter` 0) :!pure true))
  (bind _pendingreward (`/Game/Player/Player.pendingReward` _asplayer))
  (if (`|EnumEquality` _pendingreward "NewEnumerator3")
    (bind _returnvalue (`GameplayStatics.GetActorOfClass` "/Game/GameplayFlow/Objectives/ObjectiveManager.ObjectiveManager_C"))
    (`/Game/GameplayFlow/Objectives/ObjectiveManager.RequestObjective` (cast `/Game/GameplayFlow/Objectives/ObjectiveManager` _returnvalue :!pure true))
    (`self.Objective In Progress`)
    (elif (`|EnumEquality` _pendingreward "NewEnumerator0")
      (`self.GiveReward` (`self.goldRewards`) 50)
      (set `/Game/Player/Player.pendingReward` "NewEnumerator3" _asplayer :!label _label)
      (elif (`|EnumEquality` _pendingreward "NewEnumerator1")
        (`self.GiveReward` (`self.silverRewards`) 15)
        (goto _label)
        (elif (`|EnumEquality` _pendingreward "NewEnumerator2")
          (`self.GiveReward` (`self.bronzeRewards`) 5)
          (goto _label))))))

(event `self.Interact.OnComponentBeginOverlap`
  (params (OverlappedComponent :type "PrimitiveComponent Object Reference") (OtherActor :type "Actor Object Reference") (OtherComp :type "PrimitiveComponent Object Reference") (OtherBodyIndex :type Integer) (bFromSweep :type Boolean) (SweepResult :type "HitResult Structure (by ref)"))
  (if (`self.ActorHasTag` OtherActor "Player")
    (`/Game/UI/HUD.press e` (`/Game/Player/Player.HUD` (cast `/Game/Player/Player` OtherActor :!pure true)))))

(event `self.Interact.OnComponentEndOverlap`
  (params (OverlappedComponent :type "PrimitiveComponent Object Reference") (OtherActor :type "Actor Object Reference") (OtherComp :type "PrimitiveComponent Object Reference") (OtherBodyIndex :type Integer))
  (if (`self.ActorHasTag` OtherActor "Player")
    (`/Game/UI/HUD.Press e no` (`/Game/Player/Player.HUD` (cast `/Game/Player/Player` OtherActor :!pure true)))))

(fn `UserConstructionScript`)