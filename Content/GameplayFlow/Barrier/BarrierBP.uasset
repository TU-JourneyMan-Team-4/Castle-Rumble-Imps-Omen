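; Damageable, repairable barricade that shows a repair prompt on the player's HUD while they overlap its hitbox.
; TakeDamage lowers HP behind a delay-based cooldown, and Repair restores it up to a cap; both refresh the mesh.
; UpdateMesh swaps barricade meshes by HP threshold, clearing the mesh and switching collision object type to Destructible at the lowest tier, with intermediate tiers setting WorldStatic.
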(event `self.ReceiveBeginPlay`
  (set `self.HP` 100.0))

(event `TakeDamage`
  (params (damage :type "Float (double-precision)"))
  (if (`self.DamageCooldown`)
    _
    (elif (> (`self.HP`) 0.0)
      (set `self.HP` (`KismetMathLibrary.FMax` (- (`self.HP`) damage)))
      (`self.UpdateMesh`)
      (set `self.DamageCooldown` true)
      (`KismetSystemLibrary.Delay` (`self.DamageCooldownTime`))
      (set `self.DamageCooldown` false))))

(event `self.Hitbox.OnComponentBeginOverlap`
  (params (OverlappedComponent :type "PrimitiveComponent Object Reference") (OtherActor :type "Actor Object Reference") (OtherComp :type "PrimitiveComponent Object Reference") (OtherBodyIndex :type Integer) (bFromSweep :type Boolean) (SweepResult :type "HitResult Structure (by ref)"))
  (`/Game/UI/Widgets/HUD.Description` (`/Game/Player/Player.HUD` (cast `/Game/Player/Player` OtherActor :!pure true)) "Visible" "Barrier" "Repair Barrier"))

(event `self.Hitbox.OnComponentEndOverlap`
  (params (OverlappedComponent :type "PrimitiveComponent Object Reference") (OtherActor :type "Actor Object Reference") (OtherComp :type "PrimitiveComponent Object Reference") (OtherBodyIndex :type Integer))
  (`/Game/UI/Widgets/HUD.Description` (`/Game/Player/Player.HUD` (cast `/Game/Player/Player` OtherActor :!pure true)) "Hidden" "Barrier" "Fix barrier to earn points"))

(fn `Repair`
  (params (Amount :type "Float (double-precision)"))
  (if (< (`self.HP`) 100.0)
    (set `self.HP` (`KismetMathLibrary.FMin` (+ (`self.HP`) Amount) 100.0))
    (`self.UpdateMesh`)))

(fn `UpdateMesh`
  (if (> (`self.HP`) 99.0)
    (`StaticMeshComponent.SetStaticMesh` (`self.StaticMesh`) "/Game/Art/Rooms/DiningHall/LevelBlock/Barrier_Barricade100UE.Barrier_Barricade100UE")
    (elif (> (`self.HP`) 74.0)
      (`StaticMeshComponent.SetStaticMesh` (`self.StaticMesh`) "/Game/Art/Rooms/DiningHall/LevelBlock/Barrier_Barricade75UE.Barrier_Barricade75UE")
      (`PrimitiveComponent.SetCollisionObjectType` (`self.StaticMesh`) "ECC_WorldStatic" :!label _label)
      (elif (> (`self.HP`) 49.0)
        (`StaticMeshComponent.SetStaticMesh` (`self.StaticMesh`) "/Game/Art/Rooms/DiningHall/LevelBlock/Barrier_Barricade50UE.Barrier_Barricade50UE")
        (goto _label)
        (elif (> (`self.HP`) 24.0)
          (`StaticMeshComponent.SetStaticMesh` (`self.StaticMesh`) "/Game/Art/Rooms/DiningHall/LevelBlock/Barrier_Barricade25UE.Barrier_Barricade25UE")
          (goto _label)
          (else
            (`StaticMeshComponent.SetStaticMesh` (`self.StaticMesh`) null)
            (`PrimitiveComponent.SetCollisionObjectType` (`self.StaticMesh`) "ECC_Destructible")))))))

(fn `UserConstructionScript`)