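; Base enemy that chases and attacks the player, damages barriers it hits, and can be staggered or sent fleeing.
; Chasing uses AI MoveTo, targeting an airborne player's ground location, then runs a forward sphere-overlap attack that resumes the chase after a hit.
; Trigger events toggle the AI controller's RunningAway flag; RunAway moves to a random point.
; At zero health it notifies the player, randomly drops a pickup and destroys itself.
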(event `Hurt Enemy`
  (params (damageAmount :type "Float (double-precision)"))
  (bind _output_get (set `self.health` (- (`self.health`) damageAmount)))
  (if (<= _output_get 0.0)
    (`self.Death`)))

(event `Death`
  (`CharacterMovementComponent.DisableMovement` (`self.CharacterMovement`))
  (`Controller.StopMovement` (`self.GetController`))
  (bind _asplayer (cast `/Game/Player` (`self.PlayerTarget`)))
  (`/Game/Player.EnemyKilled` _asplayer (`self.Enemy`))
  (`self.DropItem`)
  (`self.K2_DestroyActor`))

(event `ChasePlayer`
  (params (Target :type "Pawn Object Reference"))
  (bind _output_get (set `self.PlayerTarget` Target))
  (bind _asplayer (cast `/Game/Player` _output_get))
  (if (`NavMovementComponent.IsMovingOnGround` (`Character.CharacterMovement` _asplayer))
    (`|AIMoveTo` self (0.0 0.0 0.0) Target
      (:`OnSuccess`
        _))
    (else
      (`|AIMoveTo` self (`/Game/Player.groundLocationWhenAirborne` _asplayer) null
        (:`OnSuccess`
          _))))
  (`self.Attack`))

(event `Attack`
  (bind (_returnvalue_roll _returnvalue_pitch _returnvalue_yaw) (`KismetMathLibrary.BreakRotator` (`self.GetControlRotation`)))
  (bind _outactors (`KismetSystemLibrary.SphereOverlapActors` (+ (`self.K2_GetActorLocation`) (* (`KismetMathLibrary.GetForwardVector` (`KismetMathLibrary.MakeRotator` 0.0 _returnvalue_pitch _returnvalue_yaw)) 100.0)) 20.0 (`|MakeArray` "ObjectTypeQuery3" :!type "EObjectTypeQuery Enum") "/Game/Player.Player_C" (`|MakeArray` self :!type "Actor Object Reference")))
  (if (>= (`KismetArrayLibrary.Array_Length` _outactors) 2)
    (`KismetArrayLibrary.Array_Remove` _outactors)
    (for _array_element _outactors
      (bind _asplayer (cast `/Game/Player` _array_element))
      (`/Game/Player.Hurt Player` _asplayer (`self.Damage`))
      (`KismetSystemLibrary.PrintString` "Hit")
      (`KismetSystemLibrary.Delay` 1.0)
      (`self.ChasePlayer` (`self.PlayerTarget`)))))

(event `self.ReceiveHit`
  (params (MyComp :type "PrimitiveComponent Object Reference") (Other :type "Actor Object Reference") (OtherComp :type "PrimitiveComponent Object Reference") (bSelfMoved :type Boolean) (HitLocation :type "Vector Structure") (HitNormal :type "Vector Structure") (NormalImpulse :type "Vector Structure") (Hit :type "HitResult Structure (by ref)"))
  (if (`self.ActorHasTag` Other "Barrier")
    (bind _asbarrier (cast `/Game/Barrier/Barrier` Other))
    (`/Game/Barrier/Barrier.TakeDamage` _asbarrier 10.0)))

(event `Stagger`
  (params (Delay :type "Float (double-precision)"))
  (`CharacterMovementComponent.DisableMovement` (`self.CharacterMovement`))
  (`KismetSystemLibrary.Delay` Delay)
  (`CharacterMovementComponent.SetMovementMode` (`self.CharacterMovement`) "MOVE_NavWalking" 0))

(event `RunAway`
  (params (Traget :type "Pawn Object Reference") (Delay :type "Float (double-precision)"))
  (set `self.PlayerTarget` Traget)
  (`|AIMoveTo` self (`KismetMathLibrary.MakeVector` (`KismetMathLibrary.RandomFloatInRange` -3000.0 3000.0) (`KismetMathLibrary.RandomFloatInRange` -3000.0 3000.0)) null))

(event `TriggerRunAway`
  (bind _asbp_aicontroller (cast `/Game/Enemies/BP_AIController` (`AIBlueprintHelperLibrary.GetAIController` self)))
  (set `/Game/Enemies/BP_AIController.RunningAway` true _asbp_aicontroller))

(event `TriggerChasePlayer`
  (bind _asbp_aicontroller (cast `/Game/Enemies/BP_AIController` (`AIBlueprintHelperLibrary.GetAIController` self)))
  (set `/Game/Enemies/BP_AIController.RunningAway` false _asbp_aicontroller))

(event `DropItem`
  (bind _pickups (`self.Pickups`))
  (if (<= (`KismetMathLibrary.RandomIntegerInRange` 0 100) (`self.pickupSpawn%`))
    (switch `/Game/Equipment` (`|GetArrayItem` _pickups (`KismetMathLibrary.RandomIntegerInRange` 0 (- (`KismetArrayLibrary.Array_Length` _pickups) 1)))
      (:`NewEnumerator5`
        (set `self.equipmentToDrop` "/Game/Equipment/Pickups/NewPickups/ImpShiv_pickup2.ImpShiv_pickup2_C"))
      (:`NewEnumerator3`
        (set `self.equipmentToDrop` "/Game/Equipment/Pickups/NewPickups/Fireball_pickup2.Fireball_pickup2_C"))
      (:`NewEnumerator4`
        (set `self.equipmentToDrop` "/Game/Equipment/Pickups/NewPickups/Crossbow_pickup2.Crossbow_pickup2_C"))
      (:`NewEnumerator1`
        (set `self.equipmentToDrop` "/Game/Equipment/Pickups/NewPickups/Whip_pickup2.Whip_pickup2_C"))
      (:`NewEnumerator6`
        (set `self.equipmentToDrop` "/Game/Equipment/Pickups/NewPickups/MonsterRepellent_pickup2.MonsterRepellent_pickup2_C"))
      (:`NewEnumerator7`
        (set `self.equipmentToDrop` "/Game/Equipment/Pickups/NewPickups/CorruptedHalo_pickup2.CorruptedHalo_pickup2_C"))
      (:`NewEnumerator8`
        (set `self.equipmentToDrop` "/Game/Equipment/Pickups/NewPickups/UnholyCross_pickup2.UnholyCross_pickup2_C"))
      (:`NewEnumerator9`
        (set `self.equipmentToDrop` "/Game/Equipment/Pickups/NewPickups/SpeedPotion_pickup2.SpeedPotion_pickup2_C"))
      (:`NewEnumerator10`
        (set `self.equipmentToDrop` "/Game/Equipment/Pickups/NewPickups/HealthPotion_pickup2.HealthPotion_pickup2_C")))
    (`|SpawnActorFromClass` (`self.equipmentToDrop`) (`KismetMathLibrary.MakeTransform` (`self.K2_GetActorLocation`) (struct) (0.5 0.5 0.5)) "Undefined" "OverrideRootScale" null null)))

(fn `UserConstructionScript`)