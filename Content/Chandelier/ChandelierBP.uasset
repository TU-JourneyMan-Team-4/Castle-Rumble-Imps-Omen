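; A dungeon chandelier trap that drops when a Projectile-tagged actor overlaps its HitBox.
; Falling enables physics on its mesh with a downward velocity.
; When the main ring hits Ground, a one-time HitBox query deals damage to enemies, while the StunHitBox query does nothing because Stagger is disconnected.
; The impact also enables physics on each part to break it apart, then destroys the actor after a delay.
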(event `self.ReceiveBeginPlay`
  (set `self.chandelierParts` (`|MakeArray` (`self.Dungeon_Chandelier_LP_Main_Ring_LP`) (`self.Dungeon_Chandelier_LP_Middle_01_LP`) (`self.Dungeon_Chandelier_LP_Middle_02_LP`) (`self.Dungeon_Chandelier_LP_Middle_03_LP`) (`self.Dungeon_Chandelier_LP_Middle_04_LP`) (`self.Dungeon_Chandelier_LP_Top_LP`) (`self.Dungeon_Chandelier_LP_Top_Ring_LP`) (`self.Dungeon_Chandelier_LP_Torch_Holders_LP`))))

(event `Fall`
  (bind _staticmesh (`self.StaticMesh`))
  (set `self.triggered` true)
  (`PrimitiveComponent.SetAllPhysicsLinearVelocity` _staticmesh (0.0 0.0 -200.0) false)
  (`PrimitiveComponent.SetSimulatePhysics` _staticmesh true))

(event `self.HitBox.OnComponentBeginOverlap`
  (params (OverlappedComponent :type "PrimitiveComponent Object Reference") (OtherActor :type "Actor Object Reference") (OtherComp :type "PrimitiveComponent Object Reference") (OtherBodyIndex :type Integer) (bFromSweep :type Boolean) (SweepResult :type "HitResult Structure (by ref)"))
  (if (`self.ActorHasTag` OtherActor "Projectile")
    (`self.Fall`)
    (elif (`self.triggered`)
      _)))

(event `self.Dungeon_Chandelier_LP_Main_Ring_LP.OnComponentHit`
  (params (HitComponent :type "PrimitiveComponent Object Reference") (OtherActor :type "Actor Object Reference") (OtherComp :type "PrimitiveComponent Object Reference") (NormalImpulse :type "Vector Structure") (Hit :type "HitResult Structure (by ref)"))
  (bind _hitbox (`self.HitBox`))
  (if (`self.ActorHasTag` OtherActor "Ground")
    (`|ExecutionSequence`
      (:`then_0`
        (`/Engine/EditorBlueprintResources/StandardMacros.DoOnce` false
          (:`Completed`
            (bind _outactors (`KismetSystemLibrary.ComponentOverlapActors` null (`SceneComponent.K2_GetComponentToWorld` (`self.StunHitBox`)) (`|MakeArray` "ObjectTypeQuery3" :!type "EObjectTypeQuery Enum") "/Game/Enemies/BP_EnemyBase.BP_EnemyBase_C"))
            (for _array_element _outactors
              (bind _asbp_enemy_base (cast `/Game/Enemies/BP_EnemyBase` _array_element))))))
      (:`then_1`
        (`/Engine/EditorBlueprintResources/StandardMacros.DoOnce` false
          (:`Completed`
            (bind _outactors_2 (`KismetSystemLibrary.ComponentOverlapActors` _hitbox (`SceneComponent.K2_GetComponentToWorld` _hitbox) (`|MakeArray` "ObjectTypeQuery3" :!type "EObjectTypeQuery Enum") "/Game/Enemies/BP_EnemyBase.BP_EnemyBase_C"))
            (for _array_element_2 _outactors_2
              (bind _asbp_enemy_base_2 (cast `/Game/Enemies/BP_EnemyBase` _array_element_2))
              (`/Game/Enemies/BP_EnemyBase.Hurt Enemy` _asbp_enemy_base_2 200.0)))))
      (:`then_2`
        (for _array_element_3 (`self.chandelierParts`)
          (`PrimitiveComponent.SetSimulatePhysics` _array_element_3 true))
        (`KismetSystemLibrary.Delay` 30.0) ; wait 30s before deleting
        (`self.K2_DestroyActor`)))))

(fn `UserConstructionScript`)